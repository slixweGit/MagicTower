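; Grid manager that builds a square or hex tile grid in its construction script.
; It sizes the collision plane and heightmap box, fills an index-to-position vector array, then optionally spawns default tiles as instanced, hierarchical or static meshes.
; An Instantiate toggle swaps flagged tile actors' meshes for instances grouped by mesh and material, or restores them.
; Gameplay grid pregeneration, terrain, wall-trace and debug-display hooks are empty stubs.
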(fn `Add Viewport Terrain To Arrays`)

(fn `Display Tile Edges Function`)

(fn `DisplayTileIndexesFunction`)

(fn `GenerateGameplayGrids`)

(fn `IndexToVectorHexGrid`
  (params (index :type Integer))
  (returns (Vector :type "Vector Structure"))
  (bind _tileboundsx (`self.TileBoundsX`))
  (return (`KismetMathLibrary.MakeVector` (+ (* (mod (/ index (`self.GridSizeX`)) 2) (/ _tileboundsx 2.0)) (* (mod index (`self.GridSizeX`)) _tileboundsx)) (* (/ index (`self.GridSizeX`)) (* (`self.TileBoundsY`) 0.75)))))

(fn `IndexToVectorSquare Grid`
  (params (Index :type Integer))
  (returns (Vector :type "Vector Structure"))
  (bind _returnvalue (/ Index (* (`self.GridSizeX`) (`self.GridSizeY`))))
  (return (`KismetMathLibrary.MakeVector` (* (mod Index (`self.GridSizeX`)) (`self.TileBoundsX`)) (* (- (/ Index (`self.GridSizeX`)) (* (`self.GridSizeX`) _returnvalue)) (`self.TileBoundsY`)) (`KismetMathLibrary.Conv_IntToDouble` (* _returnvalue 200)))))

(fn `Instances to Actors`
  (for _array_element (`self.InstanceArray`)
    (`InstancedStaticMeshComponent.ClearInstances` _array_element))
  (`KismetArrayLibrary.Array_Clear` (`self.InstanceArray`))
  (bind _outactors (`GameplayStatics.GetAllActorsOfClass` (`self.Tile Class Ref`)))
  (for _array_element_2 _outactors
    (`SceneComponent.SetVisibility` (`self.GetComponentByClass` _array_element_2 "/Script/Engine.StaticMeshComponent") true false)
    (set `/Game/MagicTower/Grid/BP_TileParent.InstanceVisibility` true _array_element_2))
  (return))

(fn `Set CollisionPlane and HeightmapBox Scale and Location`
  (returns (Location :type "Vector Structure") (`Scale X` :type "Float (double-precision)") (`Scale Y` :type "Float (double-precision)"))
  (bind _returnvalue (* (`self.TileBoundsY`) (- 1.0 (* (`KismetMathLibrary.Conv_BoolToInt` (`self.HexGrid`)) 0.25))))
  (return (+ (`self.K2_GetActorLocation`) (`KismetMathLibrary.MakeVector` (- (/ (* (+ (/ (`KismetMathLibrary.Conv_BoolToDouble` (`self.HexGrid`)) 2.0) (`KismetMathLibrary.Conv_IntToDouble` (`self.GridSizeX`))) (`self.TileBoundsX`)) 2.0) (/ (`self.TileBoundsX`) 2.0)) (- (/ (* (`self.GridSizeY`) _returnvalue) 2.0) (/ _returnvalue 2.0)) 0.1)) (* (+ (/ (`KismetMathLibrary.Conv_BoolToDouble` (`self.HexGrid`)) 2.0) (`KismetMathLibrary.Conv_IntToDouble` (`self.GridSizeX`))) (/ (`self.TileBoundsX`) 200.0)) (* (+ (`KismetMathLibrary.Conv_IntToDouble` (`self.GridSizeY`)) (* (`KismetMathLibrary.Conv_BoolToDouble` (`self.HexGrid`)) 0.25)) (/ _returnvalue 200.0))))

(fn `Trace For Walls Function`
  (params (TileIndex :type Integer) (`Debug-ShowTraces` :type Boolean)))

(fn `UserConstructionScript`
  (bind (_returnvalue_x _returnvalue_y _returnvalue_z) (`KismetMathLibrary.BreakVector` (`self.K2_GetActorLocation`)))
  (bind (_location _scale_x _scale_y) (`self.Set CollisionPlane and HeightmapBox Scale and Location`))
  (bind (_location_2 _scale_x_2 _scale_y_2) (`self.Set CollisionPlane and HeightmapBox Scale and Location`))
  (bind _instanceidtemp (`self.InstanceIDTemp`))
  (bind _defaultgridmesh (`self.DefaultGridMesh`))
  (bind _heightimpassablecutoff (`self.HeightImpassableCutoff`))
  (bind (_min _max) (`StaticMeshComponent.GetLocalBounds` (`self.Default Tile Instance`)))
  (bind _output (`|GetArrayItem` (`self.InstanceArray`) _instanceidtemp))
  (bind _returnvalue (- (* (`self.GridSizeX`) (`self.GridSizeY`) (`self.Grid Size Z`)) 1))
  (bind _returnvalue_2 (- (.y _max) (.y _min)))
  (bind _output_2 (`|GetArrayItem` (`self.K2_GetComponentsByClass` (`self.CurrentInstantiatingTile`) "/Script/Engine.StaticMeshComponent")))
  (bind (_returnvalue_location _returnvalue_rotation _returnvalue_scale) (`KismetMathLibrary.BreakTransform` (`SceneComponent.K2_GetComponentToWorld` _output_2)))
  ;[0 0.2747 1] 设置默认的网格和图块大小
  (set `self.Grid Size Squared` (* (`self.GridSizeX`) (`self.GridSizeY`)))
  (bind _returnvalue_3 (`AddComponent|NODE_AddInstancedStaticMeshComponent-0`)) ; Sets the default tile that makes up the base grid
  (set `self.Default Tile Instance` _returnvalue_3)
  (bind _returnvalue_4 (`AddComponent|NODE_AddHierarchicalInstancedStaticMeshComponent-0`))
  (set `self.Default Hierarchical Tile Instance` _returnvalue_4)
  (`SceneComponent.SetVisibility` _returnvalue_3 (`self.ShowDefaultTile`) false)
  (switch `|SwitchEnum` (`self.Default Tile Object`) ; Determines whether the grid is generated by instanced static meshes, regular static meshes (less efficient) or a texture
    (:`NewEnumerator0`
      (`StaticMeshComponent.SetStaticMesh` (`self.Default Tile Instance`) _defaultgridmesh :!label _label)
      (`StaticMeshComponent.SetStaticMesh` (`self.Default Hierarchical Tile Instance`) _defaultgridmesh)
      (set `self.TileBoundsX` (- (.x _max) (.x _min)))
      (set `self.TileBoundsY` _returnvalue_2)
      ;[1 0.2054 0] 对于六角形网格，使Y方向上的图块之间的间隙变小
      (if (`self.HexGrid`)
        (set `self.NodeGapY` (* _returnvalue_2 0.86603))
        (else
          (set `self.NodeGapY` _returnvalue_2))))
    (:`NewEnumerator2`
      (bind _output_get (set `self.TileBoundsX` (`self.GridTextureSize`)))
      (bind _output_get_2 (set `self.TileBoundsY` _output_get))
      (set `self.NodeGapY` _output_get_2)
      ;[1 1 1] 如果默认图块对象设置为纹理，则设置碰撞平面纹理（当前仅支持正方形网格）
      (bind _returnvalue_5 (`PrimitiveComponent.CreateDynamicMaterialInstance` 0 null))
      (`MaterialInstanceDynamic.SetTextureParameterValue` _returnvalue_5 "TextureParameter" (`self.DefaultTileTexture`))
      (`MaterialInstanceDynamic.SetVectorParameterValue` _returnvalue_5 "TextureSize" (make `LinearColor` (* (`self.GridSizeX`) 0.5) (* (`self.GridSizeY`) 0.5) 0.0 1.0)))
    (:`NewEnumerator3`
      (goto _label))
    (:`NewEnumerator4`
      (goto _label)))
  ;[0 0.1305 1] 缩放并定位碰撞平面。这使得不需要为平面网格设置单独的碰撞体积，并且可以在默认图块不可见的情况下在视口中放置网格
  (`SceneComponent.K2_SetWorldTransform` (`self.CollisionPlane`) (`KismetMathLibrary.MakeTransform` _location (struct) (`KismetMathLibrary.MakeVector` _scale_x _scale_y 1.0)) false false)
  (`SceneComponent.SetVisibility` (`self.CollisionPlane`) (`self.Show Collision Plane`) false)
  (switch `/Game/MagicTower/Grid/EHeight` (`self.Heightmap`)
    (:`NewEnumerator0`
      (`SceneComponent.SetVisibility` (`self.HeightmapBox`) false false))
    (:`NewEnumerator1`
      ;[0.9568 0 1] 比例和位置HeightmapBox。用于显示使用高度图跟踪的最大和最小Z位置
      (`SceneComponent.K2_SetWorldTransform` (`self.HeightmapBox`) (`KismetMathLibrary.MakeTransform` (`KismetMathLibrary.MakeVector` (.x _location_2) (.y _location_2) (+ (/ (+ (`self.Max Grid Height`) (`self.Min Grid Height`)) 2.0) _returnvalue_z)) (struct) (`KismetMathLibrary.MakeVector` _scale_x_2 _scale_y_2 (/ (- (`self.Max Grid Height`) (`self.Min Grid Height`)) 200.0))) false false :!label _label_2)
      (`SceneComponent.SetVisibility` (`self.HeightmapBox`) (`self.Show Heightmap Bounding Box`) false))
    (:`NewEnumerator2`
      (goto _label_2)))
  ;[1 0.9541 0] 创建构成网格数组索引和世界位置之间移动基础的矢量网格
  (`KismetArrayLibrary.Array_Clear` (`self.VectorFieldArray`))
  (if (`self.HexGrid`)
    (for _index (range (+ _returnvalue 1))
      (`KismetArrayLibrary.Array_Add` (`self.VectorFieldArray`) (`self.IndexToVectorHexGrid` _index)))
    (else
      (for _index_2 (range (+ _returnvalue 1))
        (`KismetArrayLibrary.Array_Add` (`self.VectorFieldArray`) (`self.IndexToVectorSquare Grid` _index_2)))))
  ;[0.21 0.21 0.21] Spawn tile grid
  (if (`self.ShowDefaultTile`)
    (switch `|SwitchEnum` (`self.Default Tile Object`)
      (:`NewEnumerator0`
        (for _array_element (`self.VectorFieldArray`)
          (`InstancedStaticMeshComponent.AddInstance` (`self.Default Tile Instance`) (`KismetMathLibrary.Conv_VectorToTransform` _array_element))))
      (:`NewEnumerator2`
        _)
      (:`NewEnumerator3`
        (for _array_element_2 (`self.VectorFieldArray`)
          (bind _returnvalue_6 (`AddComponent|NODE_AddStaticMeshComponent-0` :`RelativeTransform` (`KismetMathLibrary.Conv_VectorToTransform` _array_element_2)))
          (`StaticMeshComponent.SetStaticMesh` _returnvalue_6 (`self.DefaultGridMesh`))))
      (:`NewEnumerator4`
        (for _array_element_3 (`self.VectorFieldArray`)
          (`InstancedStaticMeshComponent.AddInstance` (`self.Default Hierarchical Tile Instance`) (`KismetMathLibrary.Conv_VectorToTransform` _array_element_3))))))
  ;[1 1 1] Prevent the user from choosing incompatible combinations of public variables
  (if (> (`self.HeightSlowIncrement`) _heightimpassablecutoff)
    (set `self.HeightSlowIncrement` _heightimpassablecutoff))
  (switch `/Game/MagicTower/Grid/EHeight` (`self.Heightmap`)
    (:`NewEnumerator0`
      _)
    (:`NewEnumerator1`
      _)
    (:`NewEnumerator2`
      (set `self.Auto Edge Costs Based on Height` true)))
  ;[0 0 0] 预生成 网格
  (if (`self.Pregenerate Gameplay Grids`)
    (`self.GenerateGameplayGrids`)
    (`PrimitiveComponent.SetCollisionEnabled` (`self.CollisionPlane`) "NoCollision")
    (`self.Add Viewport Terrain To Arrays`)
    (`PrimitiveComponent.SetCollisionEnabled` (`self.CollisionPlane`) "QueryAndPhysics")
    (if (`self.Trace for walls`)
      (for (_ _array_index) (`self.Edge Array Integer`)
        (`self.Trace For Walls Function` _array_index true)))
    (if (`self.Display Tile Indexes (Requires pregeneration)`)
      (`self.DisplayTileIndexesFunction`))
    (if (`self.Diaplay Tile Edges (Requires pregeneration)`)
      (`self.Display Tile Edges Function`)))
  ;[1 0 0.02871] 将“实例化”设置为true的角色转到视口中的实例静态网格物体，这可以大大提高性能。目前仅适用于具有单个网格和单一常规材质的演员
  (if (`self.Instantiate`)
    (set `self.IsInstantiating` true)
    (`KismetArrayLibrary.Array_Clear` (`self.InstanceArray`))
    (`KismetArrayLibrary.Array_Clear` (`self.StaticMeshArray`))
    (`KismetArrayLibrary.Array_Clear` (`self.MaterialArray`))
    (bind _outactors (`GameplayStatics.GetAllActorsOfClass` (`self.Tile Class Ref`)))
    (for _array_element_4 _outactors
      (if (`/Game/MagicTower/Grid/BP_TileParent.Instantiate` _array_element_4)
        (set `self.CurrentInstantiatingTile` _array_element_4)
        (bind _output_3 (`|GetArrayItem` (`self.K2_GetComponentsByClass` _array_element_4 "/Script/Engine.StaticMeshComponent")))
        (bind _staticmesh (`StaticMeshComponent.StaticMesh` _output_3))
        (if (`KismetArrayLibrary.Array_Contains` (`self.StaticMeshArray`) _staticmesh)
          (bind _returnvalue_7 (`PrimitiveComponent.GetMaterial` _output_3 0))
          (bind `_as材质` (cast `Material` _returnvalue_7))
          (set `self.FoundNoMaterialMatch` false)
          (for (_array_element_5 _array_index_2) (`self.StaticMeshArray`)
            (if (== _array_element_5 _staticmesh)
              (if (== (`|GetArrayItem` (`self.MaterialArray`) _array_index_2) `_as材质`)
                (set `self.InstanceIDTemp` _array_index_2)
                (set `self.FoundNoMaterialMatch` true)
                (`|ExecutionSequence`
                  (:`then_0`
                    (break))
                  (:`then_1`
                    (`PrimitiveComponent.SetMaterial` _output 0 (`|GetArrayItem` (`self.MaterialArray`) _instanceidtemp) :!label _label_3) ; Set the appropriate material and mesh before creating the instance
                    (`InstancedStaticMeshComponent.AddInstance` _output (`KismetMathLibrary.MakeTransform` (- _returnvalue_location (`self.K2_GetActorLocation`)) _returnvalue_rotation _returnvalue_scale)) ; Add instance with the same transform as the mesh of the actor
                    (`SceneComponent.SetVisibility` _output_2 false false)
                    (bind _asbp_tile_parent (cast `/Game/MagicTower/Grid/BP_TileParent` (`self.CurrentInstantiatingTile`)))
                    (set `/Game/MagicTower/Grid/BP_TileParent.InstanceVisibility` false _asbp_tile_parent))))))
          (if (not (`self.FoundNoMaterialMatch`))
            (bind `_as材质_2` (cast `Material` _returnvalue_7 :!label _label_4))
            (`KismetArrayLibrary.Array_Add` (`self.StaticMeshArray`) _staticmesh)
            (bind _returnvalue_8 (`KismetArrayLibrary.Array_Add` (`self.MaterialArray`) `_as材质_2`))
            (set `self.InstanceIDTemp` _returnvalue_8)
            (bind _returnvalue_9 (`AddComponent|NODE_AddInstancedStaticMeshComponent-1`))
            (`StaticMeshComponent.SetStaticMesh` _returnvalue_9 (`|GetArrayItem` (`self.StaticMeshArray`) (`self.InstanceIDTemp`)))
            (`KismetArrayLibrary.Array_Add` (`self.InstanceArray`) _returnvalue_9)
            (goto _label_3))
          (else
            (goto _label_4)))))
    (elif (`self.IsInstantiating`)
      (`self.Instances to Actors`)
      (set `self.IsInstantiating` false))))