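; BP_MTGameMode is the Magic Tower game mode that drives the UI flow from menu to avatar creation to main game screen.
; BeginPlay shows the menu widget, then after a short delay caches a BP_CardGameState reference.
; Req_CreateAvatar opens avatar creation, and OnAvatarCreated calls NewGame, which creates and stores the main widget.
; GameOver is empty, and PostLogin only fetches the level name on authority without using it.
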(event `self.ReceiveBeginPlay`
  (bind _returnvalue (`|CreateWidget` "/Game/MagicTower/Menu/W_Menu.W_Menu_C"))
  (`UserWidget.AddToViewport` _returnvalue 0)
  (`KismetSystemLibrary.Delay` 0.2)
  (bind _asbp_card_game_state (cast `/Game/MagicTower/Core/BP_CardGameState` (`GameplayStatics.GetGameState`)))
  (set `self.Ref_GameState` _asbp_card_game_state))

(event `Req_CreateAvatar`
  (bind _returnvalue (`|CreateWidget` "/Game/MagicTower/CreateAvatar/W_CreateAvatar.W_CreateAvatar_C"))
  (`UserWidget.AddToViewport` _returnvalue 0))

(event `OnAvatarCreated`
  (`self.NewGame`))

(event `self.K2_PostLogin`
  (params (NewPlayer :type "PlayerController Object Reference"))
  (`/Engine/EditorBlueprintResources/ActorMacros.Switch Has Authority`
    (:`Authority`
      (`GameplayStatics.GetCurrentLevelName` true))))

(event `NewGame`
  (bind _returnvalue (`|CreateWidget` "/Game/MagicTower/Core/W_Main.W_Main_C"))
  (bind _output_get (set `self.Ref_MainWidget` _returnvalue))
  (`UserWidget.AddToViewport` _output_get 0))

(event `GameOver`)

(fn `UserConstructionScript`)