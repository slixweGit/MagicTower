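; BP_PlayerAvatar is the player character Blueprint, adding a pick-up animation on a key press.
; Pressing F checks that the RefInteractive reference is valid, then plays the unarmed pick-up montage at increased speed.
; The graph neither sets that reference nor acts on the referenced object.
; BeginPlay, overlap and Tick are disabled placeholders, and the construction script only calls its parent.
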(event `Key|F`
  (params (Key :type "Key Structure"))
  (:`Pressed`
    (`/Engine/EditorBlueprintResources/StandardMacros.IsValid` (`self.Ref_Interactive`)
      (:`Is Valid`
        (`self.PlayAnimMontage` "/Game/ProgectG/Character/PickUp_noWeaponAnim_Montage.PickUp_noWeaponAnim_Montage" 3.0)))))

(fn `UserConstructionScript`
  (`parent.UserConstructionScript`))